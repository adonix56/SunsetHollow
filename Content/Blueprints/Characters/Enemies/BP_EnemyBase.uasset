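; BP_EnemyBase is a base enemy character Blueprint that plays hit-reaction montages when the enemy takes damage.
; HandleDamageAnimation picks a montage by damage type (Basic, Knockup or Knockback), falling back to the basic one if the specific montage is missing.
; It stops the current montage before playing the new one, gated by CanRestartDamageAnim and flagged with IsInDamageAnim, both reset here only when no valid montage exists.
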(event `self.BP_HandleDamageAnimation`
  (params (DamageType :type "DamageAppliedType Enum" :default "BASIC"))
  (if (`self.CanRestartDamageAnim`)
    (set `self.CanRestartDamageAnim` false)
    (set `self.IsInDamageAnim` true)
    (switch `DamageAppliedType` DamageType
      (:`BASIC`
        (bind _basicanim (`self.BasicAnim` :!label _label)
          (:`then`
            (set `self.PlayAnim` _basicanim)
            (`self.StopAnimMontage` null :!label _label_2)
            (`self.PlayAnimMontage` (`self.PlayAnim`)))
          (:`else`
            (set `self.IsInDamageAnim` false)
            (set `self.CanRestartDamageAnim` true))))
      (:`KNOCKUP`
        (bind _knockupanim (`self.KnockupAnim`)
          (:`then`
            (set `self.PlayAnim` _knockupanim)
            (goto _label_2))
          (:`else`
            (goto _label))))
      (:`KNOCKBACK`
        (bind _knockbackanim (`self.KnockbackAnim`)
          (:`then`
            (set `self.PlayAnim` _knockbackanim)
            (goto _label_2))
          (:`else`
            (goto _label)))))))

(fn `UserConstructionScript`)