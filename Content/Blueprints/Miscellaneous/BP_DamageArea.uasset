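; Hazard area that hurts a player character on overlap, or is cleared when the character passes through while invincible.
; An invincible overlap stops its four effects, fires the dashed-through event and destroys the actor after a delay.
; Otherwise it applies GE_DealDamage scaled to an attribute minus one, fires the hurt event, then later applies negative damage as apparent healing.
; The construction script tints the main effect.
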(event `self.ReceiveBeginPlay`
  (cast `SunsetHollowGameState` (`GameplayStatics.GetGameState`))
  (set `self.Deactivate` false))

(event `self.ReceiveActorBeginOverlap`
  (params (OtherActor :type "Actor Object Reference"))
  (bind _assunset_hollow_character (cast `SunsetHollowCharacter` OtherActor))
  (if (not (`self.Deactivate`))
    (bind _gascomponent (`SunsetHollowCharacter.GASComponent` _assunset_hollow_character))
    (if (`GameplayTagAssetInterface.HasMatchingGameplayTag` _gascomponent (struct :`TagName` "State.Invincible"))
      (`ActorComponent.Deactivate` (`self.DamageArea`))
      (`ActorComponent.Deactivate` (`self.DamageArea1`))
      (`ActorComponent.Deactivate` (`self.DamageArea2`))
      (`ActorComponent.Deactivate` (`self.DamageArea3`))
      (`self.OnDashedThrough`)
      (set `self.Deactivate` true)
      (`KismetSystemLibrary.Delay` 2.0)
      (`self.K2_DestroyActor`)
      (else
        (bind _returnvalue (`AbilitySystemComponent.MakeOutgoingSpec` :`self` _gascomponent :`GameplayEffectClass` "/Game/Blueprints/GAS/GameplayEffects/GE_DealDamage.GE_DealDamage_C"))
        (bind _returnvalue_2 (`AbilitySystemBlueprintLibrary.AssignTagSetByCallerMagnitude` _returnvalue (struct :`TagName` "Event.Damage") (- (`.ReturnValue` (`AbilitySystemBlueprintLibrary.GetFloatAttributeFromAbilitySystemComponent` _gascomponent (struct :`AttributeName` "Health" :`Attribute` "/Script/SunsetHollow.SunsetHollowBaseAttributeSet:Health" :`AttributeOwner` "/Script/CoreUObject.Class'/Script/SunsetHollow.SunsetHollowBaseAttributeSet'"))) 1.0)))
        (`AbilitySystemComponent.BP_ApplyGameplayEffectSpecToSelf` _gascomponent _returnvalue_2)
        (`self.OnGetHurt`)
        (`KismetSystemLibrary.Delay` 5.0)
        (bind _returnvalue_3 (`AbilitySystemBlueprintLibrary.AssignTagSetByCallerMagnitude` _returnvalue (struct :`TagName` "Event.Damage") -100.0))
        (`AbilitySystemComponent.BP_ApplyGameplayEffectSpecToSelf` _gascomponent _returnvalue_3)))))

(fn `UserConstructionScript`
  (`FXSystemComponent.SetVectorParameter` (`self.DamageArea`) "color" (`KismetMathLibrary.Conv_LinearColorToVector` (`self.ColorSlate`))))