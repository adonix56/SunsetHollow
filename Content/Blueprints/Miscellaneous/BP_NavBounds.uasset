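; BP_NavBounds is a bounds actor that moves itself away when the game reaches a configured state.
; On BeginPlay it caches its start location and binds to SunsetHollowGameState's change event.
; When the state matches GameStateToRemove, it unbinds and plays the MoveAway timeline toward EndLocation.
; Each update lerps position with a slightly randomized alpha and adds a rumble offset on X and Y for a shaking motion.
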(event `self.ReceiveBeginPlay`
  (set `self.StartLocation` (`self.K2_GetActorLocation`))
  (bind _assunset_hollow_game_state (cast `SunsetHollowGameState` (`GameplayStatics.GetGameState`)))
  (add `SunsetHollowGameState.OnGameStateChangedEvent` _assunset_hollow_game_state (delegate `OnGameStateChanged`)))

(event `OnGameStateChanged`
  (params (ChangedGameState :type "EGameState Enum" :default "NONE"))
  (if (`|EnumEquality` ChangedGameState (`self.GameStateToRemove`))
    (remove `SunsetHollowGameState.OnGameStateChangedEvent` (stale `self.ReceiveBeginPlay` _assunset_hollow_game_state) (delegate `OnGameStateChanged`))
    (bind (_direction _alpha _rumble) (`Timeline|MoveAway` :!via `PlayFromStart`)
      (:`Update`
        (bind _returnvalue (* _rumble 100.0))
        (bind _returnvalue_2 (* _alpha 0.05))
        (bind (_returnvalue_x _returnvalue_y _returnvalue_z) (`KismetMathLibrary.BreakVector` (`KismetMathLibrary.VLerp` (`self.StartLocation`) (`self.EndLocation`) (`KismetMathLibrary.RandomFloatInRange` (+ _alpha _returnvalue_2) (- _alpha _returnvalue_2)))))
        (`self.K2_SetActorLocation` (`KismetMathLibrary.MakeVector` (+ _returnvalue _returnvalue_x) (+ _returnvalue _returnvalue_y) _returnvalue_z))))))

(fn `UserConstructionScript`)