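; GA_Dash is a Gameplay Ability that dashes the owning actor toward the point under the mouse cursor.
; After committing, it traces from the deprojected cursor on the Visibility channel and turns the actor to face the hit point on the horizontal plane.
; A short constant-force root motion task then pushes the actor in that direction, ending the ability when it finishes.
; A failed commit ends the ability immediately.
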(event `self.K2_ActivateAbility`
  (bind (_worldlocation _worlddirection) (`PlayerController.DeprojectMousePositionToWorld` (`GameplayStatics.GetPlayerController` 0)))
  (bind _returnvalue (`self.K2_CommitAbility`))
  (if _returnvalue
    (bind _outhit (`KismetSystemLibrary.LineTraceSingle` _worldlocation (+ _worldlocation (* _worlddirection 5000.0)) "TraceTypeQuery1"))
    (bind (_returnvalue_x _returnvalue_y) (`KismetMathLibrary.BreakVector` (- (`.Location` (`GameplayStatics.BreakHitResult` _outhit)) (`Actor.K2_GetActorLocation` (`self.GetOwningActorFromActorInfo`)))))
    (`Actor.K2_SetActorRotation` (`self.GetOwningActorFromActorInfo`) (`KismetMathLibrary.MakeRotFromX` (`KismetMathLibrary.MakeVector` _returnvalue_x _returnvalue_y)) false)
    (`AbilityTask_ApplyRootMotionConstantForce.ApplyRootMotionConstantForce` "None" (`KismetMathLibrary.MakeVector` _returnvalue_x _returnvalue_y) 1000.0 0.25 false null "MaintainLastRootMotionVelocity"
      (:`OnFinish`
        (`self.K2_EndAbility`)))
    (else
      (`self.K2_EndAbility`))))

(event `self.K2_OnEndAbility`
  (params (bWasCancelled :type Boolean))
  (`KismetSystemLibrary.PrintString` "End Dash Ability"))