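; Gameplay Cue actor for the SuperNova visual effect, built from a main particle system and four final blast components.
; While Anim is set, Tick restarts the main particles at the RepeatBlast interval, then fires all four blasts at FinalBlast and stops.
; The start and cleanup logic in OnActive and OnRemove is disconnected, so nothing in these graphs sets Anim true or resets the timers.
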(event `self.ReceiveTick`
  (params (DeltaSeconds :type "Float (single-precision)"))
  (if (`self.Anim`)
    (bind _output_get (set `self.AnimTimeElapsed` (+ DeltaSeconds (`self.AnimTimeElapsed`))))
    (if (>= _output_get (`self.FinalBlast`))
      (`ActorComponent.SetActive` (`self.Blast1`) true true)
      (`ActorComponent.SetActive` (`self.Blast2`) true true)
      (`ActorComponent.SetActive` (`self.Blast3`) true true)
      (`ActorComponent.SetActive` (`self.Blast4`) true true)
      (set `self.Anim` false)
      (else
        (bind _output_get_2 (set `self.RepeatBlastElapsed` (+ DeltaSeconds (`self.RepeatBlastElapsed`))))
        (if (>= _output_get_2 (`self.RepeatBlast`))
          (set `self.RepeatBlastElapsed` 0.0)
          (`ActorComponent.SetActive` (`self.ParticleSystem`) true true))))))

(fn `OnActive`
  (params (MyTarget :type "Actor Object Reference") (Parameters :type "GameplayCueParameters Structure (by ref)"))
  (returns (ReturnValue :type Boolean)))

(fn `OnExecute`
  (params (MyTarget :type "Actor Object Reference") (Parameters :type "GameplayCueParameters Structure (by ref)"))
  (returns (ReturnValue :type Boolean))
  (return false))

(fn `OnRemove`
  (params (MyTarget :type "Actor Object Reference") (Parameters :type "GameplayCueParameters Structure (by ref)"))
  (returns (ReturnValue :type Boolean)))

(fn `UserConstructionScript`)