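; GA_Slash is a gameplay ability for the top-down character's montage-driven slash attack.
; After committing, it turns the character toward the cursor, plays the montage and waits for an Event.Damage gameplay event to damage the payload target.
; Montage blend-out resets the character's attack count and ends the ability, as do completion, interruption and cancellation without that reset.
; Ending clears the attacking flag and hit-enemy list.
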(event `self.K2_ActivateAbility`
  (bind _returnvalue (`self.K2_CommitAbility`))
  (if _returnvalue
    (`self.TurnCharacterTowardsCursor`)
    (`AbilityTask_PlayMontageAndWait.CreatePlayMontageAndWaitProxy` "None" (`self.Montage to Play`)
      (:`then`
        (bind (_asynctaskproxy _payload) (`AbilityTask_WaitGameplayEvent.WaitGameplayEvent` (struct :`TagName` "Event.Damage") null)
          (:`EventReceived`
            (`self.DamageEnemy` (`.Target` (break `GameplayEventData` _payload))))))
      (:`OnCompleted`
        (`self.K2_EndAbility` :!label _label))
      (:`OnBlendOut`
        (bind _asbp_top_down_character (cast `/Game/Blueprints/Characters/BP_TopDownCharacter` (`self.GetAvatarActorFromActorInfo`)))
        (set `SunsetHollowCharacter.AttackCount` 0 _asbp_top_down_character)
        (`self.K2_EndAbility`))
      (:`OnInterrupted`
        (goto _label))
      (:`OnCancelled`
        (goto _label)))
    (else
      (`self.K2_EndAbility`))))

(event `self.K2_OnEndAbility`
  (params (bWasCancelled :type Boolean))
  (bind _asbp_top_down_character (cast `/Game/Blueprints/Characters/BP_TopDownCharacter` (`self.GetAvatarActorFromActorInfo`)))
  (set `SunsetHollowCharacter.bIsAttacking` false _asbp_top_down_character)
  (`BlueprintSetLibrary.Set_Clear` (`self.HitEnemies`)))