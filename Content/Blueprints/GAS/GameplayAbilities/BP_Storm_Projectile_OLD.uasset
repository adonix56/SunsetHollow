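; Storm actor for a GAS ability that deals periodic area damage to enemies during a limited lifespan.
; BeginPlay builds one damage effect spec from the player's ability system, with negated damage as a SetByCaller magnitude.
; Tick applies that spec to enemies overlapping the Capsule at each damage interval.
; Tick also grows the Storm component to a maximum scale, then shrinks it in time for expiry, using scale over growth speed as lead time.
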(event `self.ReceiveBeginPlay`
  (`self.SetLifeSpan` (`self.Lifespan`))
  (bind _assunset_hollow_character (cast `SunsetHollowCharacter` (`Controller.K2_GetPawn` (`GameplayStatics.GetPlayerController` 0))))
  (bind _output_get (set `self.PlayerAbilitySystem` (`AbilitySystemBlueprintLibrary.GetAbilitySystemComponent` _assunset_hollow_character)))
  (bind _returnvalue (`AbilitySystemBlueprintLibrary.AssignTagSetByCallerMagnitude` (`AbilitySystemComponent.MakeOutgoingSpec` :`self` _output_get :`GameplayEffectClass` "/Game/Blueprints/GAS/GameplayEffects/GE_DealDamage.GE_DealDamage_C") (struct :`TagName` "Event.Damage") (* (`self.Damage`) -1.0)))
  (set `self.DamageSpec` _returnvalue))

(event `self.ReceiveTick`
  (params (DeltaSeconds :type "Float (single-precision)"))
  (bind _storm (`self.Storm`))
  (bind _capsule (`self.Capsule`))
  (bind _returnvalue (`SceneComponent.K2_GetComponentScale` _storm))
  (bind _returnvalue_2 (* DeltaSeconds (`self.GrowthSpeed`)))
  (bind _x (.x _returnvalue))
  (set `self.TimeSinceLastDamage` (+ (`self.TimeSinceLastDamage`) DeltaSeconds))
  (if (> (`self.TimeSinceLastDamage`) (`self.DamageInterval`))
    (bind _outactors (`KismetSystemLibrary.ComponentOverlapActors` _capsule (`SceneComponent.K2_GetComponentToWorld` _capsule) (`|MakeArray` "ObjectTypeQuery3" :!type "EObjectTypeQuery Enum") "/Script/SunsetHollow.EnemyCharacter"))
    (for _array_element _outactors
      (bind _asenemy_character (cast `EnemyCharacter` _array_element))
      (`AbilitySystemComponent.BP_ApplyGameplayEffectSpecToTarget` (`self.PlayerAbilitySystem`) (`self.DamageSpec`) (`EnemyCharacter.GASComponent` _asenemy_character)))
    (set `self.TimeSinceLastDamage` 0.0))
  (set `self.Timer` (+ (`self.Timer`) DeltaSeconds))
  (if (< (`KismetMathLibrary.SafeDivide` (`self.MaxScale`) (`self.GrowthSpeed`)) (- (`self.Lifespan`) (`self.Timer`)))
    (if (not (> _x (`self.MaxScale`)))
      (`SceneComponent.SetWorldScale3D` _storm (+ _returnvalue _returnvalue_2)))
    (elif (< _x 0.0)
      (`SceneComponent.SetWorldScale3D` (`self.Storm`) (0.0 0.0 0.0))
      (else
        (`SceneComponent.SetWorldScale3D` (`self.Storm`) (- _returnvalue (`KismetMathLibrary.Conv_DoubleToVector` _returnvalue_2)))))))

(fn `UserConstructionScript`)