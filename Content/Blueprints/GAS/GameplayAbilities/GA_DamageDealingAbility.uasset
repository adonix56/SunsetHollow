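; Base-style gameplay ability that supplies a DamageEnemy function for dealing GAS damage to enemy characters; its activate and end events are empty.
; DamageEnemy ignores non-enemies and uses the HitEnemies list so each enemy is damaged only once.
; It passes the Damage value into a GE_DealDamage spec as an Event.Damage SetByCaller magnitude, applies it to the target's ability system, and prints a debug message.
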(fn `DamageEnemy`
  (params (`Target Enemy` :type "Actor Object Reference"))
  (bind _asenemy_character (cast `EnemyCharacter` `Target Enemy`))
  (if (not (`BlueprintSetLibrary.Set_Contains` (`self.HitEnemies`) _asenemy_character))
    (`BlueprintSetLibrary.Set_Add` (`self.HitEnemies`) _asenemy_character)
    (bind _result (`/Engine/EditorBlueprintResources/StandardMacros.NegateFloat` (`self.Damage`))
      (:`  `
        (bind _returnvalue (`AbilitySystemBlueprintLibrary.AssignTagSetByCallerMagnitude` (`self.MakeOutgoingGameplayEffectSpec` "/Game/Blueprints/GAS/GameplayEffects/GE_DealDamage.GE_DealDamage_C") (struct :`TagName` "Event.Damage") _result))
        (`AbilitySystemComponent.BP_ApplyGameplayEffectSpecToTarget` (`AbilitySystemBlueprintLibrary.GetAbilitySystemComponent` (`self.GetOwningActorFromActorInfo`)) _returnvalue (`AbilitySystemBlueprintLibrary.GetAbilitySystemComponent` _asenemy_character))
        (`KismetSystemLibrary.PrintString` "Damaged Enemy!")))))