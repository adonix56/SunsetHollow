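; GA_Storm is a gameplay ability that casts a storm projectile from the player character toward the cursor.
; On activation it commits, turns the character to face the cursor and plays the storm montage.
; Shortly after the montage starts, it spawns BP_Storm_Projectile at an offset from the character, with the character's rotation and as instigator.
; The ability ends when the montage finishes or is interrupted, or if the commit fails.
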(event `self.K2_ActivateAbility`
  (`parent.K2_ActivateAbility`)
  (bind _returnvalue (`self.K2_CommitAbility`))
  (if _returnvalue
    (`self.TurnCharacterTowardsCursor`)
    (`AbilityTask_PlayMontageAndWait.CreatePlayMontageAndWaitProxy` "None" "/Game/Characters/Mannequins/Animations/AnimMontages/Storm_Montage.Storm_Montage"
      (:`then`
        (`KismetSystemLibrary.Delay` 0.2)
        (bind _assunset_hollow_character (cast `SunsetHollowCharacter` (`self.GetOwningActorFromActorInfo`)))
        (bind _returnvalue_2 (`self.GetRelativeLocationWithOffset` _assunset_hollow_character true (`self.StormSpawnOffset`)))
        (`|SpawnActorFromClass` "/Game/Blueprints/GAS/GameplayAbilities/BP_Storm_Projectile.BP_Storm_Projectile_C" (`KismetMathLibrary.MakeTransform` _returnvalue_2 (`Actor.K2_GetActorRotation` _assunset_hollow_character)) "AdjustIfPossibleButAlwaysSpawn" "MultiplyWithRoot" null _assunset_hollow_character))
      (:`OnCompleted`
        (`self.K2_EndAbility` :!label _label))
      (:`OnBlendOut`
        (goto _label))
      (:`OnInterrupted`
        (goto _label))
      (:`OnCancelled`
        (goto _label)))
    (else
      (`self.K2_EndAbility`))))