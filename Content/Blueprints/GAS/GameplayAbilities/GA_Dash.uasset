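; GA_Dash is a Gameplay Ability that dashes the top-down character toward the cursor.
; After committing, it resets the character's attack count and gets a direction from TurnCharacterTowardsCursor.
; It plays the dash montage and applies a brief constant root motion force along that direction's X and Y, ending when the force finishes.
; An unconnected inline cursor-trace rotation remains in the graph, and ending prints a debug string.
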(event `self.K2_ActivateAbility`
  (bind _returnvalue (`self.K2_CommitAbility`))
  (if _returnvalue
    (bind _asbp_top_down_character (cast `/Game/Blueprints/Characters/BP_TopDownCharacter` (`self.GetOwningActorFromActorInfo`)))
    (set `SunsetHollowCharacter.AttackCount` 0 _asbp_top_down_character)
    (bind (_outlocation _outdirection) (`self.TurnCharacterTowardsCursor`))
    (`AbilityTask_PlayMontageAndWait.CreatePlayMontageAndWaitProxy` "None" "/Game/Characters/Mannequins/Animations/AnimMontages/Dash_Montage.Dash_Montage"
      (:`then`
        (`AbilityTask_ApplyRootMotionConstantForce.ApplyRootMotionConstantForce` "None" (`KismetMathLibrary.MakeVector` (.x _outdirection) (.y _outdirection)) 1500.0 0.2 false null "MaintainLastRootMotionVelocity"
          (:`OnFinish`
            (`self.K2_EndAbility`)))))
    (else
      (`self.K2_EndAbility`))))

(event `self.K2_OnEndAbility`
  (params (bWasCancelled :type Boolean))
  (`KismetSystemLibrary.PrintString` "End Dash Ability"))