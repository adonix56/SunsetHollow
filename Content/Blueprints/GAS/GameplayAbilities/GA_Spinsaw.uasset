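; Gameplay ability for the player's Spinsaw attack, a leaping area strike aimed toward the cursor.
; On commit it turns the character, plays the montage, disables enemy collision and, after a short delay, applies GE_Spinsaw and starts a root-motion jump.
; Damage events trigger a sphere trace around the instigator that damages enemies not in HitEnemies, then clears that list.
; Jump completion or montage end finishes the ability, restoring collision.
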(event `self.K2_ActivateAbility`
  (bind _returnvalue (`self.K2_CommitAbility`))
  (if _returnvalue
    (bind (_outlocation _outdirection) (`self.TurnCharacterTowardsCursor`))
    (`AbilityTask_PlayMontageAndWait.CreatePlayMontageAndWaitProxy` "None" "/Game/Characters/Mannequins/Animations/AnimMontages/Spinsaw_Montage.Spinsaw_Montage"
      (:`then`
        (bind _assunset_hollow_character (cast `SunsetHollowCharacter` (`self.GetOwningActorFromActorInfo`)))
        (`SunsetHollowCharacter.IgnoreEnemyCollision` _assunset_hollow_character true)
        (`AbilityTask_WaitDelay.WaitDelay` 0.26
          (:`OnFinish`
            (`self.BP_ApplyGameplayEffectToOwner` "/Game/Blueprints/GAS/GameplayEffects/GE_Spinsaw.GE_Spinsaw_C")
            (bind _returnvalue_2 (`self.GetRotatorDirectionFromVector` _outdirection))
            (`AbilityTask_ApplyRootMotionJumpForce.ApplyRootMotionJumpForce` "None" _returnvalue_2 500.0 200.0 0.42 0.0 false "MaintainLastRootMotionVelocity"
              (:`then`
                (bind (_asynctaskproxy _payload) (`AbilityTask_WaitGameplayEvent.WaitGameplayEvent` (struct :`TagName` "Event.Damage") null)
                  (:`EventReceived`
                    (bind _returnvalue_3 (`Actor.K2_GetActorLocation` (`.Instigator` (break `GameplayEventData` _payload))))
                    (bind _outhits (`KismetSystemLibrary.SphereTraceMultiForObjects` :`Start` _returnvalue_3 :`End` _returnvalue_3 :`Radius` 125.0 :`ObjectTypes` (`|MakeArray` "ObjectTypeQuery3" :!type "EObjectTypeQuery Enum") :`DrawDebugType` "ForDuration"))
                    (for _array_element _outhits
                      (bind _asenemy_character (cast `EnemyCharacter` (`.HitActor` (`GameplayStatics.BreakHitResult` _array_element))))
                      (if (not (`BlueprintSetLibrary.Set_Contains` (`self.HitEnemies`) _asenemy_character))
                        (`self.DamageEnemy` _asenemy_character)))
                    (`BlueprintSetLibrary.Set_Clear` (`self.HitEnemies`)))))
              (:`OnFinish`
                (`self.K2_EndAbility`))))))
      (:`OnCompleted`
        (`self.K2_EndAbility` :!label _label))
      (:`OnInterrupted`
        (goto _label))
      (:`OnCancelled`
        (goto _label)))
    (else
      (`self.K2_EndAbility`))))

(event `self.K2_OnEndAbility`
  (params (bWasCancelled :type Boolean))
  (`parent.K2_OnEndAbility` bWasCancelled)
  (bind _assunset_hollow_character (cast `SunsetHollowCharacter` (`self.GetOwningActorFromActorInfo`)))
  (`SunsetHollowCharacter.IgnoreEnemyCollision` _assunset_hollow_character false))