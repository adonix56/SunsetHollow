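; SuperNova gameplay ability that pulls nearby enemies toward the caster with repeated damage pulses, then blasts them outward.
; On commit, it faces the cursor, plays the montage, applies GE_SuperNova to the owner and, after a short delay, adjusts camera zoom.
; A delayed loop of capsule traces deals basic damage, skipping the pull on enemies already close.
; When repeats run out, a final trace deals knockback damage; montage end or interruption ends the ability.
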(event `self.K2_ActivateAbility`
  (bind _repeat_count (`self.Repeat Count`))
  (bind _returnvalue (`Actor.K2_GetActorLocation` (`self.GetOwningActorFromActorInfo`)))
  (`parent.K2_ActivateAbility`)
  (bind _returnvalue_2 (`self.K2_CommitAbility`))
  (if _returnvalue_2
    (`self.TurnCharacterTowardsCursor`)
    (`AbilityTask_PlayMontageAndWait.CreatePlayMontageAndWaitProxy` "None" "/Game/Characters/Mannequins/Animations/AnimMontages/Supernova_Montage.Supernova_Montage"
      (:`then`
        (bind _assunset_hollow_character (cast `SunsetHollowCharacter` (`self.GetOwningActorFromActorInfo`)))
        (`self.BP_ApplyGameplayEffectToOwner` "/Game/Blueprints/GAS/GameplayEffects/GE_SuperNova.GE_SuperNova_C")
        (`AbilityTask_WaitDelay.WaitDelay` 0.4
          (:`then`
            (bind _returnvalue_3 (`self.GetRelativeLocationWithOffset` (`self.GetOwningActorFromActorInfo`)))
            (bind _outhits (`KismetSystemLibrary.CapsuleTraceMultiForObjects` _returnvalue_3 _returnvalue_3 300.0 300.0 (`|MakeArray` "ObjectTypeQuery3" :!type "EObjectTypeQuery Enum") :!label _label))
            (for _array_element _outhits
              (bind _asenemy_character (cast `EnemyCharacter` (`.HitActor` (`GameplayStatics.BreakHitResult` _array_element))))
              (if (not (`BlueprintSetLibrary.Set_Contains` (`self.HitEnemies`) _asenemy_character))
                (bind _returnvalue_4 (`Actor.K2_GetActorLocation` _asenemy_character))
                (if (> (`KismetMathLibrary.Vector_Distance2DSquared` _returnvalue_4 _returnvalue) 10000.0)
                  (set `self.MoveDistance` 500.0)
                  (else
                    (set `self.MoveDistance` 0.0)))
                (`self.DamageEnemy` _asenemy_character "BASIC" (`self.Repeat Damage`) (`self.MoveDistance`) (`KismetMathLibrary.Vector_Normal2D` (- _returnvalue _returnvalue_4)))))
            (`BlueprintSetLibrary.Set_Clear` (`self.HitEnemies`))
            (`AbilityTask_WaitDelay.WaitDelay` (`self.RepeatDelay`)
              (:`OnFinish`
                (if (> _repeat_count 0)
                  (set `self.Repeat Count` (- _repeat_count 1))
                  (goto _label)
                  (else
                    (bind _outhits_2 (`KismetSystemLibrary.CapsuleTraceMultiForObjects` _returnvalue_3 _returnvalue_3 300.0 300.0 (`|MakeArray` "ObjectTypeQuery3" :!type "EObjectTypeQuery Enum")))
                    (for _array_element_2 _outhits_2
                      (bind _asenemy_character_2 (cast `EnemyCharacter` (`.HitActor` (`GameplayStatics.BreakHitResult` _array_element_2))))
                      (if (not (`BlueprintSetLibrary.Set_Contains` (`self.HitEnemies`) _asenemy_character_2))
                        (`self.DamageEnemy` _asenemy_character_2 "KNOCKBACK" (`self.Blast Damage`) 2000.0 (`KismetMathLibrary.Vector_Normal2D` (- (`Actor.K2_GetActorLocation` _asenemy_character_2) (`Actor.K2_GetActorLocation` (`self.GetOwningActorFromActorInfo`)))))))
                    (`BlueprintSetLibrary.Set_Clear` (`self.HitEnemies`)))))))
          (:`OnFinish`
            (`SunsetHollowCharacter.ZoomCameraWithTimer` _assunset_hollow_character 0.3 500.0 0.0 1.0))))
      (:`OnCompleted`
        (`self.K2_EndAbility` :!label _label_2))
      (:`OnInterrupted`
        (goto _label_2))
      (:`OnCancelled`
        (goto _label_2)))
    (else
      (`self.K2_EndAbility`))))