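; Gameplay ability for the bat enemy's attack, currently turning it to face the player and printing a debug message.
; On activation it commits the ability, then reads the Player character from the enemy's blackboard to use as the turn target.
; The ability ends only when the commit fails; the successful path applies no damage and never calls EndAbility.
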(event `self.K2_ActivateAbility`
  (bind _returnvalue (`self.K2_CommitAbility`))
  (if _returnvalue
    (bind _asenemy_character (cast `EnemyCharacter` (`self.GetOwningActorFromActorInfo`)))
    (bind _assunset_hollow_character (cast `SunsetHollowCharacter` (`BlackboardComponent.GetValueAsObject` (`AIBlueprintHelperLibrary.GetBlackboard` _asenemy_character) "Player")))
    (`self.TurnTowardsActor` _assunset_hollow_character)
    (`KismetSystemLibrary.PrintString` "Enemy Bat Attacking!")
    (else
      (`self.K2_EndAbility`))))