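; Player Guillotine ability: a montage-driven lunge toward the cursor that damages and knocks back enemies.
; Constant-force root motion moves the character with enemy collision ignored until the ability ends, and a shockwave emitter spawns shortly after launch.
; Montage-timed gameplay events apply GE_Guillotine on the thunder event and run capsule traces on each damage event.
; Hits after the first trace at an offset location, pushing enemies away from the player.
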(event `self.K2_ActivateAbility`
  (`parent.K2_ActivateAbility`)
  (bind _returnvalue (`self.K2_CommitAbility`))
  (if _returnvalue
    (set `self.FirstHit` true)
    (bind (_outlocation _outdirection) (`self.TurnCharacterTowardsCursor`))
    (`AbilityTask_PlayMontageAndWait.CreatePlayMontageAndWaitProxy` "None" "/Game/Characters/Mannequins/Animations/AnimMontages/Guillotine_Montage.Guillotine_Montage" 1.0 "None" false
      (:`then`
        (bind _assunset_hollow_character (cast `SunsetHollowCharacter` (`self.GetOwningActorFromActorInfo`)))
        (`SunsetHollowCharacter.IgnoreEnemyCollision` _assunset_hollow_character true)
        (`AbilityTask_ApplyRootMotionConstantForce.ApplyRootMotionConstantForce` "None" (`KismetMathLibrary.MakeVector` (.x _outdirection) (.y _outdirection)) 300.0 0.89 false null "MaintainLastRootMotionVelocity"
          (:`then`
            (`AbilityTask_WaitDelay.WaitDelay` 0.1
              (:`then`
                (`AbilityTask_WaitGameplayEvent.WaitGameplayEvent` (struct :`TagName` "Event.GuillotineThunder") null
                  (:`then`
                    (bind (_asynctaskproxy _payload) (`AbilityTask_WaitGameplayEvent.WaitGameplayEvent` (struct :`TagName` "Event.Damage") null)
                      (:`EventReceived`
                        (bind _returnvalue_2 (`self.GetRelativeLocationWithOffset` (`.Instigator` (break `GameplayEventData` _payload)) (not (`self.FirstHit`)) (`self.Offset`)))
                        (set `self.FirstHit` false)
                        (bind _outhits (`KismetSystemLibrary.CapsuleTraceMultiForObjects` _returnvalue_2 _returnvalue_2 80.0 200.0 (`|MakeArray` "ObjectTypeQuery3" :!type "EObjectTypeQuery Enum")))
                        (for _array_element _outhits
                          (bind _asenemy_character (cast `EnemyCharacter` (`.HitActor` (`GameplayStatics.BreakHitResult` _array_element))))
                          (if (not (`BlueprintSetLibrary.Set_Contains` (`self.HitEnemies`) _asenemy_character))
                            (`self.DamageEnemy` _asenemy_character "KNOCKBACK" 20.0 1500.0 (`KismetMathLibrary.Vector_Normal2D` (- (`Actor.K2_GetActorLocation` _asenemy_character) (`Actor.K2_GetActorLocation` (`self.GetOwningActorFromActorInfo`)))))))
                        (`BlueprintSetLibrary.Set_Clear` (`self.HitEnemies`)))))
                  (:`EventReceived`
                    (`self.BP_ApplyGameplayEffectToOwner` "/Game/Blueprints/GAS/GameplayEffects/GE_Guillotine.GE_Guillotine_C"))))
              (:`OnFinish`
                (`GameplayStatics.SpawnEmitterAttached` "/Game/FX/P_ky_shotShockwave.P_ky_shotShockwave" (`Actor.RootComponent` (`self.GetOwningActorFromActorInfo`)) "None" (0.0 0.0 0.0) (struct :`Pitch` 90.0)))))))
      (:`OnCompleted`
        (`self.K2_EndAbility`)))
    (else
      (`self.K2_EndAbility`))))

(event `self.K2_OnEndAbility`
  (params (bWasCancelled :type Boolean))
  (`parent.K2_OnEndAbility` bWasCancelled)
  (bind _assunset_hollow_character (cast `SunsetHollowCharacter` (`self.GetOwningActorFromActorInfo`)))
  (`SunsetHollowCharacter.IgnoreEnemyCollision` _assunset_hollow_character false))