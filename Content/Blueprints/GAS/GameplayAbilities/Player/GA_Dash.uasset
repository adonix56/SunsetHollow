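; Player dash gameplay ability that lunges the Sunset Hollow character toward the cursor.
; Once committed, it resets the attack count, turns the character to the cursor, plays the dash montage and disables enemy collision.
; A short constant root motion force drives the movement; its finish, rather than the montage's, ends the ability, and OnEndAbility restores enemy collision.
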(event `self.K2_ActivateAbility`
  (bind _returnvalue (`self.K2_CommitAbility`))
  (if _returnvalue
    (bind _assunset_hollow_character (cast `SunsetHollowCharacter` (`self.GetOwningActorFromActorInfo`)))
    (set `SunsetHollowCharacter.AttackCount` 0 _assunset_hollow_character)
    (bind (_outlocation _outdirection) (`self.TurnCharacterTowardsCursor`))
    (`AbilityTask_PlayMontageAndWait.CreatePlayMontageAndWaitProxy` "None" "/Game/Characters/Mannequins/Animations/AnimMontages/Dash_Montage.Dash_Montage"
      (:`then`
        (`SunsetHollowCharacter.IgnoreEnemyCollision` _assunset_hollow_character true)
        (`AbilityTask_ApplyRootMotionConstantForce.ApplyRootMotionConstantForce` "None" (`KismetMathLibrary.MakeVector` (.x _outdirection) (.y _outdirection)) 1500.0 0.2 false null "MaintainLastRootMotionVelocity"
          (:`OnFinish`
            (`self.K2_EndAbility`)))))
    (else
      (`self.K2_EndAbility`))))

(event `self.K2_OnEndAbility`
  (params (bWasCancelled :type Boolean))
  (bind _assunset_hollow_character (cast `SunsetHollowCharacter` (`self.GetOwningActorFromActorInfo`)))
  (`SunsetHollowCharacter.IgnoreEnemyCollision` _assunset_hollow_character false))