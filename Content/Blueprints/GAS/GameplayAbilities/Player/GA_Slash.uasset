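; GA_Slash is the player's slash attack, a Gameplay Ability in the Gameplay Ability System.
; After committing, it turns the character toward the cursor and plays an attack montage while waiting for an Event.Damage gameplay event.
; A received event damages the targeted EnemyCharacter with BASIC damage.
; Montage blend-out resets the character's AttackCount and ends the ability, while completion, interruption, cancellation or a failed commit simply end it.
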(event `self.K2_ActivateAbility`
  (bind _returnvalue (`self.K2_CommitAbility`))
  (if _returnvalue
    (`self.TurnCharacterTowardsCursor`)
    (`AbilityTask_PlayMontageAndWait.CreatePlayMontageAndWaitProxy` "None" (`self.Montage to Play`)
      (:`then`
        (bind (_asynctaskproxy _payload) (`AbilityTask_WaitGameplayEvent.WaitGameplayEvent` (struct :`TagName` "Event.Damage") null)
          (:`EventReceived`
            (bind _asenemy_character (cast `EnemyCharacter` (`.Target` (break `GameplayEventData` _payload))))
            (`KismetSystemLibrary.PrintString` "Hit Enemy")
            (`self.DamageEnemy` _asenemy_character "BASIC" (`self.Damage`)))))
      (:`OnCompleted`
        (`self.K2_EndAbility` :!label _label))
      (:`OnBlendOut`
        (bind _assunset_hollow_character (cast `SunsetHollowCharacter` (`self.GetAvatarActorFromActorInfo`)))
        (set `SunsetHollowCharacter.AttackCount` 0 _assunset_hollow_character)
        (`self.K2_EndAbility`))
      (:`OnInterrupted`
        (goto _label))
      (:`OnCancelled`
        (goto _label)))
    (else
      (`self.K2_EndAbility`))))

(event `self.K2_OnEndAbility`
  (params (bWasCancelled :type Boolean))
  (`parent.K2_OnEndAbility` bWasCancelled))